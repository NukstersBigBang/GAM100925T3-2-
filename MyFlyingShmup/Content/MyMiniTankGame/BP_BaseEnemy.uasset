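; Base enemy Blueprint for the mini tank game, with health, a widget health bar and a death effect.
; On overlap it damages the other actor by its own current health.
; Incoming damage reduces clamped health and updates the bar percentage through a widget cast, which must succeed before the death check runs.
; At zero health it calls DestroyActor, then OnDeath plays a sound, spawns an explosion and calls DestroyActor again.
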(event `self.ReceiveBeginPlay`
  (set `self.Health` (`self.MaxHealth`)))

(event `self.ReceiveActorBeginOverlap`
  (params (OtherActor :type "Actor Object Reference"))
  (`GameplayStatics.ApplyDamage` OtherActor (`self.Health`)))

(event `self.ReceiveAnyDamage`
  (params (Damage :type "Float (single-precision)") (DamageType :type "DamageType Object Reference") (InstigatedBy :type "Controller Object Reference") (DamageCauser :type "Actor Object Reference"))
  (set `self.Health` (`KismetMathLibrary.FClamp` (- (`self.Health`) Damage) 0.0 (`self.MaxHealth`)))
  (bind _aswbd_enemy_health_bar (cast `/Game/MyMiniTankGame/UI/WBD_EnemyHealthBar` (`WidgetComponent.GetUserWidgetObject` (`self.Widget`))))
  (`/Game/MyMiniTankGame/UI/WBD_EnemyHealthBar.SetHealthAsPercent` _aswbd_enemy_health_bar (`KismetMathLibrary.SafeDivide` (`self.Health`) (`self.MaxHealth`)))
  (`self.CheckHealth`))

(event `CheckHealth`
  (if (== (`self.Health`) 0.0)
    (`self.K2_DestroyActor`)
    (`self.OnDeath`)))

(event `OnDeath`
  (`GameplayStatics.PlaySound2D` "/Game/MyMiniTankGame/Audio/hit-windy-thud-399086.hit-windy-thud-399086" 1.0 1.0 0.0 null null)
  (`self.SpawnExplosion`)
  (`self.K2_DestroyActor`))

(event `SpawnExplosion`
  (`NiagaraFunctionLibrary.SpawnSystemAtLocation` "/Game/MyMiniTankGame/VFX/FX_EnemyExplosion_System.FX_EnemyExplosion_System" (`self.K2_GetActorLocation`)))

(fn `UserConstructionScript`)