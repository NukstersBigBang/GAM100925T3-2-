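; Player pawn that moves, fires bullets, takes damage and respawns through Gamemode_MyFlyingShmup on death.
; W/A/S/D toggle Gates polled on Tick for thrust and turning, alongside Enhanced Input axis movement and delayed single-shot fire.
; Spawn grants two seconds without box collision; overlaps damage both actors, and damage triggers camera shake and a health check.
; Alternate shooting modes are left disconnected, and the hit-flash event is never called here.
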(event `self.ReceiveBeginPlay`
  (`PrimitiveComponent.SetCollisionEnabled` (`self.Box`) "NoCollision")
  (`KismetSystemLibrary.Delay` 2.0)
  (`PrimitiveComponent.SetCollisionEnabled` (`self.Box`) "QueryAndPhysics")
  (set `self.PlayerHealth` (`self.MaxHealth`)))

(event `self.ReceiveTick`
  (params (DeltaSeconds :type "Float (single-precision)"))
  ; Movement
  (`|ExecutionSequence`
    (:`then_0`
      (`/Engine/EditorBlueprintResources/StandardMacros.Gate` true :!label _label
        (:`Exit`
          (`PawnMovementComponent.AddInputVector` (`self.FloatingPawnMovement`) (`self.GetActorForwardVector`) false))))
    (:`then_1`
      (`/Engine/EditorBlueprintResources/StandardMacros.Gate` true :!label _label_2
        (:`Exit`
          (`self.K2_AddActorLocalRotation` (struct :`Yaw` -0.3))
          (`KismetSystemLibrary.Delay` 0.4)
          (`self.K2_AddActorLocalRotation` (struct :`Yaw` 0.5)))))
    (:`then_2`
      (`/Engine/EditorBlueprintResources/StandardMacros.Gate` true :!label _label_3
        (:`Exit`
          (`PawnMovementComponent.AddInputVector` (`self.FloatingPawnMovement`) (* (`self.GetActorForwardVector`) (-1.0 -1.0 -1.0)) false))))
    (:`then_3`
      (`/Engine/EditorBlueprintResources/StandardMacros.Gate` true :!label _label_4
        (:`Exit`
          (`self.K2_AddActorLocalRotation` (struct :`Yaw` 0.3))
          (`KismetSystemLibrary.Delay` 0.4)
          (`self.K2_AddActorLocalRotation` (struct :`Yaw` -0.5)))))))

(event `Key|W`
  (params (Key :type "Key Structure"))
  ; Movement
  (:`Pressed`
    (goto _label :!via `Open`))
  (:`Released`
    (goto _label :!via `Close`)))

(event `self.ReceivePossessed`
  (params (NewController :type "Controller Object Reference"))
  ; Movement (2)
  (bind _asplayer_controller (cast `PlayerController` NewController))
  (`EnhancedInputSubsystemInterface.AddMappingContext` (pcsubsystem `EnhancedInputLocalPlayerSubsystem` _asplayer_controller) "/Game/MyMiniTankGame/Inputs/IMC_PlayerMovement.IMC_PlayerMovement" 0 (struct)))

(event `Key|S`
  (params (Key :type "Key Structure"))
  ; Movement
  (:`Pressed`
    (goto _label_3 :!via `Open`))
  (:`Released`
    (goto _label_3 :!via `Close`)))

(event `Key|A`
  (params (Key :type "Key Structure"))
  ; Movement
  (:`Pressed`
    (goto _label_2 :!via `Open`))
  (:`Released`
    (goto _label_2 :!via `Close`)))

(event `EnhancedInput|/Game/MyMiniTankGame/Inputs/IA_MoveRightLeft`
  (params (ActionValue :type "Float (double-precision)") (ElapsedSeconds :type "Float (double-precision)") (TriggeredSeconds :type "Float (double-precision)") (InputAction :type "InputAction Object Reference" :default "/Game/MyMiniTankGame/Inputs/IA_MoveRightLeft.IA_MoveRightLeft"))
  ; Movement (2)
  (:`Triggered`
    (`PawnMovementComponent.AddInputVector` (`self.FloatingPawnMovement`) (`KismetMathLibrary.MakeVector` 0.0 ActionValue) false)))

(event `Key|D`
  (params (Key :type "Key Structure"))
  ; Movement
  (:`Pressed`
    (goto _label_4 :!via `Open`))
  (:`Released`
    (goto _label_4 :!via `Close`)))

(event `EnhancedInput|/Game/MyMiniTankGame/Inputs/IA_MoveUpDown`
  (params (ActionValue :type "Float (double-precision)") (ElapsedSeconds :type "Float (double-precision)") (TriggeredSeconds :type "Float (double-precision)") (InputAction :type "InputAction Object Reference" :default "/Game/MyMiniTankGame/Inputs/IA_MoveUpDown.IA_MoveUpDown"))
  ; Movement (2)
  (:`Triggered`
    (`PawnMovementComponent.AddInputVector` (`self.FloatingPawnMovement`) (`KismetMathLibrary.MakeVector` 0.0 0.0 ActionValue) false)))

(event `EnhancedInput|/Game/MyMiniTankGame/Inputs/IA_PrimaryFire`
  (params (ActionValue :type Boolean) (ElapsedSeconds :type "Float (double-precision)") (TriggeredSeconds :type "Float (double-precision)") (InputAction :type "InputAction Object Reference" :default "/Game/MyMiniTankGame/Inputs/IA_PrimaryFire.IA_PrimaryFire"))
  (bind (_returnvalue_location _returnvalue_rotation) (`KismetMathLibrary.BreakTransform` (`SceneComponent.K2_GetComponentToWorld` (`self.Shooting1`))))
  (:`Triggered`
    (`KismetSystemLibrary.Delay` 0.2)
    ; Shooting Mode 1
    (`|SpawnActorFromClass` "/Game/MyMiniTankGame/BP_BulletPlayer.BP_BulletPlayer_C" (`KismetMathLibrary.MakeTransform` _returnvalue_location _returnvalue_rotation) "Undefined" "MultiplyWithRoot" null null)))

(event `self.ReceiveAnyDamage`
  (params (Damage :type "Float (single-precision)") (DamageType :type "DamageType Object Reference") (InstigatedBy :type "Controller Object Reference") (DamageCauser :type "Actor Object Reference"))
  (set `self.PlayerHealth` (`KismetMathLibrary.FClamp` (- (`self.PlayerHealth`) Damage) 0.0 (`self.MaxHealth`)))
  (`self.ApplyCameraShake`)
  (`self.CheckHealth`))

(event `self.ReceiveActorBeginOverlap`
  (params (OtherActor :type "Actor Object Reference"))
  (`|ExecutionSequence`
    (:`then_0`
      (`GameplayStatics.ApplyDamage` OtherActor (`self.PlayerHealth`)))
    (:`then_1`
      (`GameplayStatics.ApplyDamage` self (`self.Damage`)))))

(event `CheckHealth`
  (if (== (`self.PlayerHealth`) 0.0)
    (`self.OnDeath`)))

(event `ApplyCameraShake`
  (`GameplayStatics.PlayWorldCameraShake` "/Game/MyMiniTankGame/BP_CameraShake.BP_CameraShake_C" (0.0 0.0 0.0) 0.0 100000.0))

(event `FlashingWhenAttacked`
  (`MeshComponent.SetOverlayMaterial` (`self.Cube2`) null)
  (`KismetSystemLibrary.Delay` 0.2)
  (`MeshComponent.SetOverlayMaterial` (`self.Cube2`) null))

(event `OnDeath`
  (bind _asgamemode_my_flying_shmup (cast `/Game/MyMiniTankGame/Core/Gamemode_MyFlyingShmup` (`GameplayStatics.GetGameMode`)))
  (`/Game/MyMiniTankGame/Core/Gamemode_MyFlyingShmup.RespawnPlayer` _asgamemode_my_flying_shmup self)
  (`self.K2_DestroyActor`))

(fn `UserConstructionScript`)