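; BP_HomingEnemy is a shoot 'em up enemy that turns toward the player and fires a bullet.
; A timer set on BeginPlay triggers the EaseFacePlayer timeline, which interpolates the actor's yaw toward the player pawn on each update.
; When the timeline finishes, it spawns BP_BulletEnemy at the Arrow component's location and rotation, so the shot follows the new facing.
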(event `self.ReceiveBeginPlay`
  (`self.StartShooting`))

(event `StartShooting`
  (`KismetSystemLibrary.K2_SetTimerDelegate` (delegate `FacePlayer`) 2.0))

(event `FacePlayer`
  (bind (_returnvalue_roll _returnvalue_pitch _returnvalue_yaw) (`KismetMathLibrary.BreakRotator` (`KismetMathLibrary.FindLookAtRotation` (`self.K2_GetActorLocation`) (`self.K2_GetActorLocation` (`GameplayStatics.GetPlayerPawn` 0)))))
  (`Timeline|EaseFacePlayer`
    (:`Update`
      (bind _output_get (set `self.TargetYaw` _returnvalue_yaw))
      (bind (_returnvalue_roll_2 _returnvalue_pitch_2 _returnvalue_yaw_2) (`KismetMathLibrary.BreakRotator` (`KismetMathLibrary.RInterpTo` (`KismetMathLibrary.MakeRotator` 0.0 0.0 (`self.CurrentYaw`)) (`KismetMathLibrary.MakeRotator` 0.0 0.0 _output_get) (`GameplayStatics.GetWorldDeltaSeconds`))))
      (bind _output_get_2 (set `self.CurrentYaw` _returnvalue_yaw_2))
      (`self.K2_SetActorRotation` (`KismetMathLibrary.MakeRotator` 0.0 0.0 _output_get_2)))
    (:`Finished`
      (`self.FireBullet`))))

(event `FireBullet`
  (bind _arrow (`self.Arrow`))
  (`|SpawnActorFromClass` "/Game/SHMUP_Game/Blueprint/BP_BulletEnemy.BP_BulletEnemy_C" (`KismetMathLibrary.MakeTransform` (`SceneComponent.K2_GetComponentLocation` _arrow) (`SceneComponent.K2_GetComponentRotation` _arrow)) "Undefined" "MultiplyWithRoot" null null))

(fn `UserConstructionScript`
  (`parent.UserConstructionScript`))