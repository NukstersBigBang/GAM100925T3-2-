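; BP_WaveSpawner is an actor that endlessly spawns random enemies for the SHMUP game.
; From BeginPlay, a self-requeuing timer fires SpawnEnemy after a short random delay.
; Each spawn picks a class from EnemyTypes and a random Y position between the ArrowLeft and ArrowRight markers, using ArrowLeft's X, Z and rotation.
; Random picks draw on random streams, with Stream reset at BeginPlay.
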(event `self.ReceiveBeginPlay`
  (`KismetMathLibrary.ResetRandomStream` (`self.Stream`))
  (`self.QueueTimer`))

(event `QueueTimer`
  (`KismetSystemLibrary.K2_SetTimerDelegate` (delegate `SpawnEnemy`) (`KismetMathLibrary.RandomFloatInRangeFromStream` (`self.Stream_0`) 1.0 3.0)))

(event `SpawnEnemy`
  (bind _arrow__left_ (`self.Arrow (Left)`))
  (bind (_returnvalue_x _returnvalue_y) (`KismetMathLibrary.BreakVector` (`SceneComponent.K2_GetComponentLocation` (`self.Arrow (Right)`))))
  (bind (_returnvalue_x_2 _returnvalue_y_2 _returnvalue_z) (`KismetMathLibrary.BreakVector` (`SceneComponent.K2_GetComponentLocation` _arrow__left_)))
  (`|SpawnActorFromClass` (`KismetArrayLibrary.Array_RandomFromStream` (`self.EnemyTypes`) (`self.Stream`)) (`KismetMathLibrary.MakeTransform` (`KismetMathLibrary.MakeVector` _returnvalue_x_2 (`KismetMathLibrary.RandomFloatInRangeFromStream` (`self.Stream_0`) _returnvalue_y_2 _returnvalue_y) _returnvalue_z) (`SceneComponent.K2_GetComponentRotation` _arrow__left_)) "Undefined" "MultiplyWithRoot" null null)
  (`self.QueueTimer`))

(fn `UserConstructionScript`)